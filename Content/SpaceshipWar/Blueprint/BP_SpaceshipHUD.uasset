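; BP_SpaceshipHUD is the spaceship game's HUD Blueprint, which shows or hides the WBP_HUD widget.
; ToggleAllElementsVisibility lazily creates the widget for the owning player controller on first show, caches it in HUDWidgetRef, and adds it to the viewport.
; Hiding removes the cached widget from its parent if it is in the viewport, keeping the reference for reuse.
; The event graph and construction script contain no active logic.
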(event EventBeginPlay)

(event Collision|EventActorBeginOverlap
  (params (OtherActor :type Actor%20Object%20Reference)))

(event EventTick
  (params (DeltaSeconds :type Float%20%28single-precision%29)))

(fn ConstructionScript)

(fn ToggleAllElementsVisibility
  (params (InToggleFlag :type Boolean))
  (if InToggleFlag
    (Utilities|IsValid (Variables|Default|GetHUDWidgetRef)
      (:Is%20Valid
        _)
      (:Is%20Not%20Valid
        (bind _returnvalue (UserInterface|CreateWidget "/Game/SpaceshipWar/UI/WBP_HUD.WBP_HUD_C" (Game|Player|GetOwningPlayerController)))
        (Variables|Default|SetHUDWidgetRef _returnvalue)))
    (UserInterface|Viewport|AddtoViewport (Variables|Default|GetHUDWidgetRef) 0)
    (else
      (Utilities|IsValid (Variables|Default|GetHUDWidgetRef)
        (:Is%20Valid
          (if (UserInterface|Viewport|IsinViewport (Variables|Default|GetHUDWidgetRef))
            (Widget|RemovefromParent (Variables|Default|GetHUDWidgetRef))))))))