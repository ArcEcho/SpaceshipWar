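; Game mode for a two-player spaceship duel that runs rounds from login through results and rematch.
; PostLogin records controllers and starts when two players join; RestartRound resets HP and respawns each ship at its index-tagged PlayerStart.
; EndRound waits one second so in-flight bullets can cause a draw, then shows results, scores the winner and destroys pawns.
; A new round starts once both players are ready.
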(event Custom|EndRound
  ;[1 1 1] The round will be over if one of the player is killed
  (if (not (Variables|Default|GetIsRoundEnd))
    (Variables|Default|SetIsRoundEnd true)
    ;;[1 1 1] Delay to check the result for flying bullet , allow drawn round
    (Utilities|FlowControl|Delay 1.0)
    (CallFunction|RoundResultCheck)
    (for _array_element (Variables|Default|GetPlayerList)
      (bind _asbp_spaceship_player_state (Utilities|Casting|CastToBP_SpaceshipPlayerState (Variables|/Script/Engine.Controller|GetPlayerState _array_element)))
      (Variables|/Game/SpaceshipWar/Blueprint/BP_SpaceshipPlayerState.BP_SpaceshipPlayerState_C|SetIsReady _asbp_spaceship_player_state false)
      (Utilities|IsValid (Pawn|GetControlledPawn _array_element)
        (:Is%20Valid
          (Actor|DestroyActor (Pawn|GetControlledPawn _array_element)))))))

(event Custom|ResetPlayer
  (params (InPlayer :type BP%20Spaceship%20Player%20Controller%20Object%20Reference))
  (bind _returnvalue (Pawn|GetControlledPawn InPlayer))
  ;[1 1 1] Reset player current HP
  (bind _asbp_spaceship_player_state (Utilities|Casting|CastToBP_SpaceshipPlayerState (Variables|/Script/Engine.Controller|GetPlayerState InPlayer))
    (:then
      (Variables|/Game/SpaceshipWar/Blueprint/BP_SpaceshipPlayerState.BP_SpaceshipPlayerState_C|SetIsReady _asbp_spaceship_player_state false)
      (Variables|/Game/SpaceshipWar/Blueprint/BP_SpaceshipPlayerState.BP_SpaceshipPlayerState_C|SetCurrentHP _asbp_spaceship_player_state 100)
      ;[1 1 1] Destroy the origin pawn an spawn a new one at a desired PlayerStart.
      (Utilities|IsValid _returnvalue
        (:Is%20Valid
          (Actor|DestroyActor _returnvalue))
        (:Is%20Not%20Valid
          _))
      (bind _outactors (Actor|GetAllActorswithTag (Utilities|String|StringToName (Utilities|String|Append "PlayerStart_" (Utilities|String|ToString(Integer) (Utilities|Array|FindItem (Variables|Default|GetPlayerList) InPlayer))))))
      (bind _returnvalue_2 (Game|SpawnActorfromClass "/Game/SpaceshipWar/Blueprint/BP_Spaceship.BP_Spaceship_C" (Transformation|GetActorTransform (Utilities|Array|Get(acopy) _outactors)) "Undefined" 0 0))
      (Pawn|Possess InPlayer _returnvalue_2))
    (:CastFailed
      (Development|PrintString "GameMode cast PlayerState  failed"))))

(event Custom|RestartRound
  ;[1 1 1] Restart Round
  (Variables|Default|SetIsRoundEnd false)
  (for _array_element (Variables|Default|GetPlayerList)
    (CallFunction|ResetPlayer _array_element)
    (Default|ClientShowRoundStartCountDownWidget _array_element)))

(event Custom|OnPlayerReadyToRestartRound
  (params (InPlayer :type Controller%20Object%20Reference))
  (bind _asbp_spaceship_player_state (Utilities|Casting|CastToBP_SpaceshipPlayerState (Variables|/Script/Engine.Controller|GetPlayerState InPlayer)))
  (Variables|/Game/SpaceshipWar/Blueprint/BP_SpaceshipPlayerState.BP_SpaceshipPlayerState_C|SetIsReady _asbp_spaceship_player_state true)
  ;[1 1 1] Check whether if both players are ready to restart round
  (bind _asbp_spaceship_player_state_2 (Utilities|Casting|CastToBP_SpaceshipPlayerState (Variables|/Script/Engine.Controller|GetPlayerState (Utilities|Array|Get(acopy) (Variables|Default|GetPlayerList)))))
  (bind _asbp_spaceship_player_state_3 (Utilities|Casting|CastToBP_SpaceshipPlayerState (Variables|/Script/Engine.Controller|GetPlayerState (Utilities|Array|Get(acopy) (Variables|Default|GetPlayerList) 1))))
  (if (Variables|/Game/SpaceshipWar/Blueprint/BP_SpaceshipPlayerState.BP_SpaceshipPlayerState_C|GetIsReady _asbp_spaceship_player_state_2)
    (if (Variables|/Game/SpaceshipWar/Blueprint/BP_SpaceshipPlayerState.BP_SpaceshipPlayerState_C|GetIsReady _asbp_spaceship_player_state_3)
      (CallFunction|RestartRound))))

(event EventBeginPlay)

(event EventTick
  (params (DeltaSeconds :type Float%20%28single-precision%29)))

(event EventPostLogin
  (params (NewPlayer :type Player%20Controller%20Object%20Reference))
  ;[1 1 1] Record player on player login
  (bind _asbp_spaceship_player_controller (Utilities|Casting|CastToBP_SpaceshipPlayerController NewPlayer)
    (:then
      (Utilities|Array|AddUnique (Variables|Default|GetPlayerList) _asbp_spaceship_player_controller)
      (bind _returnvalue (Class|GameModeBase|GetNumPlayers))
      (if (== _returnvalue 2)
        ;[1 1 1] If 2 player has login in the game , the game should start, otherwise show waiting message
        (CallFunction|RestartRound)
        (else
          (Default|ShowWaitforAnOpponentWidget _asbp_spaceship_player_controller))))
    (:CastFailed
      (Development|PrintString "OnPostLogin: cast to desired PlayerController failed"))))

(fn ConstructionScript)

(fn RoundResultCheck
  (bind _playerlist (Variables|Default|GetPlayerList))
  (bind _playerlist_2 (Variables|Default|GetPlayerList))
  ;[1 1 1] Get player's HP value
  (bind _asbp_spaceship_player_state (Utilities|Casting|CastToBP_SpaceshipPlayerState (Variables|/Script/Engine.Controller|GetPlayerState (Utilities|Array|Get(acopy) (Variables|Default|GetPlayerList)))))
  (LocalVariables|SetPlayer1StateRef _asbp_spaceship_player_state)
  (bind _asbp_spaceship_player_state_2 (Utilities|Casting|CastToBP_SpaceshipPlayerState (Variables|/Script/Engine.Controller|GetPlayerState (Utilities|Array|Get(acopy) (Variables|Default|GetPlayerList) 1))))
  (LocalVariables|SetPlayer2StateRef _asbp_spaceship_player_state_2)
  (if (and (== 0 (Variables|/Game/SpaceshipWar/Blueprint/BP_SpaceshipPlayerState.BP_SpaceshipPlayerState_C|GetCurrentHP (LocalVariables|GetPlayer1StateRef))) (== 0 (Variables|/Game/SpaceshipWar/Blueprint/BP_SpaceshipPlayerState.BP_SpaceshipPlayerState_C|GetCurrentHP (LocalVariables|GetPlayer2StateRef))))
    (for _array_element (Variables|Default|GetPlayerList)
      (Default|ClientShowRoundResult _array_element "Drawn round!"))
    (elif (!= (Variables|/Game/SpaceshipWar/Blueprint/BP_SpaceshipPlayerState.BP_SpaceshipPlayerState_C|GetCurrentHP (LocalVariables|GetPlayer1StateRef)) 0)
      (CallFunction|DispatchLoseandWinRoundResult (Utilities|Array|Get(acopy) _playerlist_2) (Utilities|Array|Get(acopy) _playerlist_2 1))
      (else
        (CallFunction|DispatchLoseandWinRoundResult (Utilities|Array|Get(acopy) _playerlist 1) (Utilities|Array|Get(acopy) _playerlist))))))

(fn DispatchLoseandWinRoundResult
  (params (InWinner :type BP%20Spaceship%20Player%20Controller%20Object%20Reference) (InLoser :type BP%20Spaceship%20Player%20Controller%20Object%20Reference))
  (Default|ClientShowRoundResult InWinner "Win!")
  (bind _asbp_spaceship_player_state (Utilities|Casting|CastToBP_SpaceshipPlayerState (Variables|/Script/Engine.Controller|GetPlayerState InWinner)))
  (Default|IncreasePlayerScore _asbp_spaceship_player_state)
  (Default|ClientShowRoundResult InLoser "Lose!"))