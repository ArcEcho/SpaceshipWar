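; Player controller for a multiplayer spaceship battle that manages round-flow UI and input modes.
; On begin play it views through the tagged MainCamera, yawed to match the controller's rotation.
; Client events show countdown and result widgets, creating each once, and toggle HUD visibility and cursor; another shows a waiting-for-opponent widget.
; A server event forwards the player's readiness to restart the round to BP_BattleGameMode.
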(event Custom|Server_AttemptToRestartRound
  (bind _asbp_battle_game_mode (Utilities|Casting|CastToBP_BattleGameMode (Game|GetGameMode)))
  (Default|OnPlayerReadytoRestartRound _asbp_battle_game_mode self)
  (Utilities|Casting|CastToBP_SpaceshipHUD (HUD|GetHUD)))

(event Custom|Client_ShowRoundResult
  (params (RoundResult :type String))
  (Utilities|FlowControl|Delay 1.0)
  (Utilities|IsValid (Variables|Default|GetRoundResultWidget)
    (:Is%20Valid
      _)
    (:Is%20Not%20Valid
      (bind _returnvalue (UserInterface|CreateWidget "/Game/SpaceshipWar/UI/WBP_RoundResult.WBP_RoundResult_C" self))
      (Variables|Default|SetRoundResultWidget _returnvalue)))
  (UserInterface|Viewport|AddtoViewport (Variables|Default|GetRoundResultWidget) 0)
  (Default|SetRoundResult (Variables|Default|GetRoundResultWidget) RoundResult)
  (Variables|Default|SetbShowMouseCursor true)
  (Input|SetInputModeUIOnly self 0 "DoNotLock")
  (bind _asbp_spaceship_hud (Utilities|Casting|CastToBP_SpaceshipHUD (HUD|GetHUD)))
  (Default|ToggleAllElementsVisibility _asbp_spaceship_hud false))

(event Custom|ShowWaitForAnOpponentWidget
  (Utilities|IsValid (Variables|Default|GetWaitForAnOpponentWidget)
    (:Is%20Valid
      _)
    (:Is%20Not%20Valid
      (bind _returnvalue (UserInterface|CreateWidget "/Game/SpaceshipWar/UI/WBP_WaitForAnOpponentWidget.WBP_WaitForAnOpponentWidget_C" self))
      (Variables|Default|SetWaitForAnOpponentWidget _returnvalue)))
  (UserInterface|Viewport|AddtoViewport (Variables|Default|GetWaitForAnOpponentWidget) 0)
  (Variables|Default|SetbShowMouseCursor false)
  (Input|SetInputModeUIOnly self 0 "DoNotLock")
  (Utilities|Casting|CastToBP_SpaceshipHUD (HUD|GetHUD)))

(event Custom|Client_ShowRoundStartCountDownWidget
  (bind _waitforanopponentwidget (Variables|Default|GetWaitForAnOpponentWidget))
  (Utilities|IsValid (Variables|Default|GetRoundStartCountDownWidget)
    (:Is%20Valid
      _)
    (:Is%20Not%20Valid
      (bind _returnvalue (UserInterface|CreateWidget "/Game/SpaceshipWar/UI/WBP_RoundStartCountDownWidget.WBP_RoundStartCountDownWidget_C" self))
      (Variables|Default|SetRoundStartCountDownWidget _returnvalue)))
  (UserInterface|Viewport|AddtoViewport (Variables|Default|GetRoundStartCountDownWidget) 0)
  (Utilities|IsValid _waitforanopponentwidget
    (:Is%20Valid
      (if (UserInterface|Viewport|IsinViewport _waitforanopponentwidget)
        (Widget|RemovefromParent _waitforanopponentwidget)
        (Variables|Default|SetbShowMouseCursor false)
        (Input|SetInputModeUIOnly self 0 "DoNotLock")
        (bind _asbp_spaceship_hud (Utilities|Casting|CastToBP_SpaceshipHUD (HUD|GetHUD)))
        (Default|ToggleAllElementsVisibility _asbp_spaceship_hud false)))))

(event Custom|Client_OnCountDownEnd
  (bind _asbp_spaceship_hud (Utilities|Casting|CastToBP_SpaceshipHUD (HUD|GetHUD)))
  (Default|ToggleAllElementsVisibility _asbp_spaceship_hud true)
  (Variables|Default|SetbShowMouseCursor false)
  (Input|SetInputModeGameOnly self))

(event EventBeginPlay
  (Input|SetInputModeGameOnly self)
  ;[1 1 1] Set the orientation of the main camera
  (bind _outactors (Actor|GetAllActorswithTag "MainCamera"))
  (Transformation|SetActorRotation (Utilities|Array|Get(acopy) _outactors) (Math|Rotator|MakeRotator (.Roll (Math|Rotator|BreakRotator (Transformation|GetActorRotation (Utilities|Array|Get(acopy) _outactors)))) (.Pitch (Math|Rotator|BreakRotator (Transformation|GetActorRotation (Utilities|Array|Get(acopy) _outactors)))) (.Yaw (Math|Rotator|BreakRotator (Transformation|GetActorRotation)))))
  (Game|Player|SetViewTargetwithBlend (Utilities|Array|Get(acopy) _outactors) 0.0 "VTBlend_Linear" 0.0 false))

(fn ConstructionScript)

(fn ShowRoundResultWidget
  (Utilities|IsValid (Variables|Default|GetRoundResultWidget)
    (:Is%20Valid
      _)
    (:Is%20Not%20Valid
      (bind _returnvalue (UserInterface|CreateWidget "/Game/SpaceshipWar/UI/WBP_RoundResult.WBP_RoundResult_C" self))
      (Variables|Default|SetRoundResultWidget _returnvalue)))
  (UserInterface|Viewport|AddtoViewport (Variables|Default|GetRoundResultWidget) 0)
  (Variables|Default|SetbShowMouseCursor true)
  (Input|SetInputModeUIOnly self 0 "DoNotLock"))

(fn NeedUIOperation
  (params (IsNeeded :type Boolean))
  (bind _self self)
  (Variables|Default|SetbShowMouseCursor IsNeeded)
  (if IsNeeded
    (Input|SetInputModeUIOnly _self 0 "DoNotLock")
    (else
      (Input|SetInputModeGameOnly _self))))