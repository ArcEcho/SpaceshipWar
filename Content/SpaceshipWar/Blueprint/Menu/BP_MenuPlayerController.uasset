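; Player controller for the SpaceshipWar front-end menu that switches between the startup, main menu, server list and options screens.
; TransitMenuPhase removes the current phase's widget from the viewport, records the new phase, then shows that phase's widget, creating it on first use and caching it for reuse.
; BeginPlay prints the player and display names for debugging, and SetPlayerName is an empty stub.
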(event EventBeginPlay
  (Development|PrintString (Variables|/Script/Engine.PlayerState|GetPlayerName (Variables|GetPlayerState self)))
  (Development|PrintString (Utilities|GetDisplayName 0)))

(event EventTick
  (params (DeltaSeconds :type Float%20%28single-precision%29)))

(fn ConstructionScript)

(fn SetPlayerName
  (params (InPlayerName :type String)))