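; Player-controlled multiplayer spaceship pawn that flies to its start position, then enables sideways movement and firing.
; Tick interpolates strafe speed and banks the mesh; axis input is applied locally and sent to the server.
; Timer-throttled fire calls the server to spawn bullets, with client RPCs for effects.
; Damage reduces PlayerState HP; death destroys the ship and ends the GameMode round, while a delayed check assigns player or enemy material.
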(event Custom|Client_OnKilled
  (bind _returnvalue (Transformation|GetActorLocation))
  ;[1 1 1] Player is killed
  (Rendering|SetActorHiddenInGame true)
  (Effects|SpawnEmitteratLocation "/Game/SpaceshipWar/Particles/P_Pixel_Explosion_Player.P_Pixel_Explosion_Player" _returnvalue)
  (Audio|PlaySoundatLocation "/Game/SpaceshipWar/Audio/A_Explosion.A_Explosion" _returnvalue)
  (Camera|PlayWorldCameraShake "/Game/SpaceshipWar/Blueprint/BP_SpaceshipExplosionCameraShake.BP_SpaceshipExplosionCameraShake_C" _returnvalue 0.0 5e+02))

(event Custom|UpdateMoveRightInputAxisValue
  (params (HozMoveDirection :type Float%20%28single-precision%29))
  ;[1 1 1] Handle movement input
  (Variables|Default|SetHozMoveDirection HozMoveDirection))

(event Custom|Server_UpdateMoveRightInputAxisValue
  (params (HozMoveDirection :type Float%20%28single-precision%29))
  ;[1 1 1] Handle movement input
  (CallFunction|UpdateMoveRightInputAxisValue HozMoveDirection))

(event Custom|Server_Fire
  (bind _bulletspawnposition (Variables|Default|GetBulletSpawnPosition))
  (bind _returnvalue (Transformation|GetWorldLocation _bulletspawnposition))
  ;[1 1 1] Handle fire action input
  (Game|SpawnActorfromClass "/Game/SpaceshipWar/Blueprint/BP_Bullet.BP_Bullet_C" (Math|Transform|MakeTransform _returnvalue (Transformation|GetActorRotation)) "Undefined" 0 0)
  (CallFunction|ClientPlayFireSound _returnvalue))

(event Custom|ContinousFire
  ;[1 1 1] Handle fire action input
  (Variables|Default|SetCanFire true)
  (if (Variables|Default|GetIsFireActionActivated)
    (CallFunction|ServerFire)
    (Variables|Default|SetCanFire false)
    (else
      (Utilities|Time|ClearandInvalidateTimerbyHandle (Variables|Default|GetFireTimerHandle)))))

(event Custom|Client_PlayFireSound
  (params (Location :type Vector))
  ;[1 1 1] Handle fire action input
  (Audio|PlaySoundatLocation "/Game/SpaceshipWar/Audio/A_Shot.A_Shot" Location))

(event EventBeginPlay
  (bind _returnvalue (Transformation|GetActorForwardVector))
  ;[1 1 1] Calculate desired location for starting game
  (Variables|Default|SetDisiredLocation (+ (Transformation|GetActorLocation) (* _returnvalue 1.5e+02)))
  ;[1 1 1] Set engine trail emitter inital veloctiy
  (Effects|Components|ParticleSystem|SetVectorParameter (Variables|Default|GetP_EngineTrail) "Direction" (Math|Vector|MakeVector 0.0 0.0 (* (.X (Math|Vector|BreakVector _returnvalue)) -2e+02)))
  ;[1 1 1] Do not use  delay
  (Utilities|Time|SetTimerbyFunctionName 0 "SetSpaceshipMaterial" 1.0))

(event EventTick
  (params (DeltaSeconds :type Float%20%28single-precision%29))
  (bind _returnvalue (Transformation|GetActorLocation))
  (bind _spaceshipmeshsceneroot (Variables|Default|GetSpaceshipMeshSceneRoot))
  (bind _disiredlocation (Variables|Default|GetDisiredLocation))
  (bind _returnvalue_2 (- _disiredlocation _returnvalue))
  (bind _returnvalue_3 (Math|Vector|VectorLength _returnvalue_2))
  ;[1 1 1] Move forward to the desired location
  (if (Variables|Default|GetIsInputEnabled)
    ;[1 1 1] Tick movement
    (bind _returndirection (CallFunction|Movement (Variables|Default|GetHozSpeed) (Variables|Default|GetHozMoveDirection) DeltaSeconds))
    (bind _output_get (Variables|Default|SetHozSpeed _returndirection))
    (Transformation|AddActorWorldOffset (* (Transformation|GetActorRightVector) _output_get) true)
    (Transformation|SetRelativeRotation _spaceshipmeshsceneroot (Class|KismetMathLibrary|RInterptoConstant (Variables|/Script/Engine.SceneComponent|GetRelativeRotation _spaceshipmeshsceneroot) (Math|Rotator|MakeRotator (* (Variables|Default|GetHozSpeed) 2e+01) 0.0 0.0) DeltaSeconds 4e+01) false false)
    (else
      (Transformation|AddActorWorldOffset (* (* (Transformation|GetActorForwardVector) DeltaSeconds) (Variables|Default|GetSpeed)) true)
      (if (or (<= _returnvalue_3 1.0) (>= _returnvalue_3 155.0))
        (Variables|Default|SetIsInputEnabled true)
        (Transformation|SetActorLocation (Variables|Default|GetDisiredLocation) false true)))))

(event Game|Damage|EventAnyDamage
  (params (Damage :type Float%20%28single-precision%29) (DamageType :type Damage%20Type%20Object%20Reference) (InstigatedBy :type Controller%20Object%20Reference) (DamageCauser :type Actor%20Object%20Reference))
  ;[1 1 1] Handle damage taking
  (bind _asbp_spaceship_player_state (Utilities|Casting|CastToBP_SpaceshipPlayerState (Variables|GetPlayerState)))
  (if (> (- (Variables|/Game/SpaceshipWar/Blueprint/BP_SpaceshipPlayerState.BP_SpaceshipPlayerState_C|GetCurrentHP _asbp_spaceship_player_state) (Math|Float|Truncate Damage)) 0)
    (Variables|/Game/SpaceshipWar/Blueprint/BP_SpaceshipPlayerState.BP_SpaceshipPlayerState_C|SetCurrentHP _asbp_spaceship_player_state (- (Variables|/Game/SpaceshipWar/Blueprint/BP_SpaceshipPlayerState.BP_SpaceshipPlayerState_C|GetCurrentHP _asbp_spaceship_player_state) (Math|Float|Truncate Damage)))
    (else
      (Variables|/Game/SpaceshipWar/Blueprint/BP_SpaceshipPlayerState.BP_SpaceshipPlayerState_C|SetCurrentHP _asbp_spaceship_player_state 0)
      (Pawn|UnPossess (Pawn|GetController self))
      (Collision|SetCollisionEnabled (Variables|Default|GetBox) "NoCollision")
      (CallFunction|ClientonKilled)
      (Utilities|FlowControl|Delay 0.2)
      (Actor|DestroyActor)
      (bind _asbp_battle_game_mode (Utilities|Casting|CastToBP_BattleGameMode (Game|GetGameMode)))
      (Default|EndRound _asbp_battle_game_mode))))

(event Input|ActionEvents|InputActionFire
  (params (Key :type Key%20Structure :default "AnyKey"))
  ;[1 1 1] Handle fire action input
  (:Pressed
    (if (Variables|Default|GetIsInputEnabled)
      (Variables|Default|SetIsFireActionActivated true)
      (if (Variables|Default|GetCanFire)
        (CallFunction|ServerFire)
        (Variables|Default|SetCanFire false)
        (bind _returnvalue (Utilities|Time|SetTimerbyEvent (delegate Custom|ContinousFire) 0.5 true))
        (Variables|Default|SetFireTimerHandle _returnvalue))))
  (:Released
    (Variables|Default|SetIsFireActionActivated false)))

(event Input|AxisEvents|InputAxisMoveRight
  (params (AxisValue :type Float%20%28single-precision%29))
  ;[1 1 1] Handle movement input
  (Networking|SwitchHasAuthority
    (:Authority
      (CallFunction|UpdateMoveRightInputAxisValue AxisValue))
    (:Remote
      (CallFunction|ServerUpdateMoveRightInputAxisValue AxisValue)
      (CallFunction|UpdateMoveRightInputAxisValue AxisValue))))

(fn ConstructionScript)

(fn Movement
  (params (Speed :type Float%20%28single-precision%29) (Direction :type Float%20%28single-precision%29) (DeltaTime :type Float%20%28single-precision%29))
  (bind _output_get (Variables|Default|SetCurrentSpeed (Math|Interpolation|FInterpTo Speed (* Direction (Variables|Default|GetMovementSpeed)) DeltaTime 4.0)))
  (return _output_get))

(fn SetSpaceshipMaterial
  (bind _staticmesh (Variables|Default|GetStaticMesh))
  (if (!= (Pawn|GetControlledPawn (Game|GetPlayerController 0)) self)
    (Rendering|Material|SetMaterial _staticmesh 0 "/Game/SpaceshipWar/Material/MI_Spaceship_Enemy.MI_Spaceship_Enemy")
    (else
      (Rendering|Material|SetMaterial _staticmesh 0 "/Game/SpaceshipWar/Material/MI_Spaceship_Player.MI_Spaceship_Player"))))