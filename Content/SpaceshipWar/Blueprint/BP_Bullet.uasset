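; BP_Bullet is a networked spaceship projectile that damages any BP_Spaceship it hits.
; Each tick, the authority calls ClientMove and remotes call ServerMove, which forwards to ClientMove for a swept forward offset.
; On hit, the authority applies damage and triggers the client explosion event, which hides the bullet and plays particles and sound.
; It then disables collision and destroys the actor after a short delay.
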(event OnComponentHit(Box)
  (params (HitComponent :type Primitive%20Component%20Object%20Reference) (OtherActor :type Actor%20Object%20Reference) (OtherComp :type Primitive%20Component%20Object%20Reference) (NormalImpulse :type Vector :default "0, 0, 0") (Hit :type Hit%20Result%20Structure%20%28by%20ref%29))
  (bind (_bblockinghit _binitialoverlap _time _location _impactpoint _normal _impactnormal _physmat _hitactor) (Collision|BreakHitResult Hit))
  ;[1 1 1] Handle collision
  (Networking|SwitchHasAuthority
    (:Authority
      (bind _asbp_spaceship (Utilities|Casting|CastToBP_Spaceship _hitactor)
        (:then
          (Game|Damage|ApplyDamage _asbp_spaceship (Variables|Default|GetDamage) 0 self))
        (:CastFailed
          _))
      (CallFunction|ClientPlayBullletExplosionEffect _location)
      (Collision|SetCollisionEnabled (Variables|Default|GetBox) "NoCollision")
      (Utilities|FlowControl|Delay 0.2)
      (Actor|DestroyActor))))

(event Custom|Server_Move
  (params (InDeltaTime :type Float%20%28single-precision%29))
  ;[1 1 1] Handle bullet movement
  (CallFunction|ClientMove InDeltaTime))

(event Custom|Client_PlayBullletExplosionEffect
  (params (Location :type Vector))
  ;[1 1 1] Play client side effect
  (Rendering|SetActorHiddenInGame true)
  (Effects|SpawnEmitteratLocation "/Game/SpaceshipWar/Particles/P_Pixel_Explosion.P_Pixel_Explosion" Location)
  (Audio|PlaySoundatLocation "/Game/SpaceshipWar/Audio/A_Explosion.A_Explosion" Location))

(event Custom|Client_Move
  (params (InDeltaTime :type Float%20%28single-precision%29))
  ;[1 1 1] Handle bullet movement
  (Transformation|AddActorWorldOffset (* (Transformation|GetActorForwardVector) (* InDeltaTime (Variables|Default|GetMoveSpeed))) true))

(event EventBeginPlay)

(event Collision|EventActorBeginOverlap
  (params (OtherActor :type Actor%20Object%20Reference)))

(event EventTick
  (params (DeltaSeconds :type Float%20%28single-precision%29))
  ;[1 1 1] Handle bullet movement
  (Networking|SwitchHasAuthority
    (:Authority
      (CallFunction|ClientMove DeltaSeconds))
    (:Remote
      (CallFunction|ServerMove DeltaSeconds))))

(fn ConstructionScript)