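; Game instance for SpaceshipWar that manages menu screens, stores the player's name, and reports multiplayer errors.
; Show events add the main menu, server list and options widgets to the viewport, creating and caching each one when no valid instance exists.
; Travel and network failure handlers print readable messages, with most network failure types grouped as lost connection, timeout or other error.
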(event Custom|ShowMainMenu
  (Utilities|IsValid (Variables|MenuWidget|GetMainMenuWIdget)
    (:Is%20Valid
      (UserInterface|Viewport|AddtoViewport (Variables|MenuWidget|GetMainMenuWIdget) 0))
    (:Is%20Not%20Valid
      (bind _returnvalue (UserInterface|CreateWidget "/Game/SpaceshipWar/UI/Menu/WBP_MainMenu.WBP_MainMenu_C" (Game|GetPlayerController 0)))
      (bind _output_get (Variables|MenuWidget|SetMainMenuWIdget _returnvalue))
      (UserInterface|Viewport|AddtoViewport _output_get 0))))

(event Custom|ShowOption
  (Utilities|IsValid (Variables|MenuWidget|GetOptionsWidget)
    (:Is%20Valid
      (UserInterface|Viewport|AddtoViewport (Variables|MenuWidget|GetOptionsWidget) 0))
    (:Is%20Not%20Valid
      (bind _returnvalue (UserInterface|CreateWidget "/Game/SpaceshipWar/UI/Menu/WBP_Options.WBP_Options_C" (Game|GetPlayerController 0)))
      (bind _output_get (Variables|MenuWidget|SetOptionsWidget _returnvalue))
      (UserInterface|Viewport|AddtoViewport _output_get 0))))

(event Custom|ShowServerList
  (Utilities|IsValid (Variables|MenuWidget|GetServerListVidgit)
    (:Is%20Valid
      (UserInterface|Viewport|AddtoViewport (Variables|MenuWidget|GetServerListVidgit) 0))
    (:Is%20Not%20Valid
      (bind _returnvalue (UserInterface|CreateWidget "/Game/SpaceshipWar/UI/Menu/WBP_MenuServerList.WBP_MenuServerList_C" (Game|GetPlayerController 0)))
      (bind _output_get (Variables|MenuWidget|SetServerListVidgit _returnvalue))
      (UserInterface|Viewport|AddtoViewport _output_get 0))))

(event EventHandleTravelError
  (params (FailureType :type ETravelFailure%20Enum))
  (bind _returnvalue (CallFunction|TravelErrortoString FailureType))
  (Development|PrintString _returnvalue))

(event EventHandleNetworkError
  (params (FailureType :type ENetworkFailure%20Enum) (bIsServer :type Boolean))
  (bind _outstring (CallFunction|NetworkErrortoString FailureType))
  (Development|PrintString _outstring))

(fn SetPlayerName
  (params (InPlayerName :type String))
  (Variables|Default|SetPlayerName InPlayerName))

(fn GetPlayerName
  (return (Variables|Default|GetPlayerName)))

(fn TravelErrortoString
  (params (ErrorType :type ETravelFailure%20Enum))
  (return (Utilities|String|Append "Error: failed to travel. " (Utilities|String|EnumtoString ErrorType))))

(fn NetworkErrortoString
  (params (InErrorType :type ENetworkFailure%20Enum))
  (switch Utilities|FlowControl|Switch|SwitchonENetworkFailure InErrorType
    (:NetDriverAlreadyExists
      (LocalVariables|SetErrorString "Error: lost connection to host." :!label _label))
    (:NetDriverCreateFailure
      (goto _label))
    (:NetDriverListenFailure
      (goto _label))
    (:ConnectionLost
      (goto _label))
    (:ConnectionTimeout
      (LocalVariables|SetErrorString "Error: connection timed out."))
    (:FailureReceived
      (goto _label))
    (:OutdatedClient
      (goto _label))
    (:OutdatedServer
      (goto _label))
    (:PendingConnectionFailure
      (goto _label))
    (:NetGuidMismatch
      (LocalVariables|SetErrorString "Error: other network error." :!label _label_2))
    (:NetChecksumMismatch
      (goto _label_2)))
  (return (LocalVariables|GetErrorString)))